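; Child enemy Blueprint that extends its parent enemy with a ranged shot attack.
; On BeginPlay it runs the parent logic, then attaches the Casting component to the mesh's CastingPoint socket.
; The ShotBall event spawns a Shot at the enemy's own transform rather than the socket, then destroys it after a short delay if still valid.
; Nothing in this graph calls ShotBall.
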(event Custom|ShotBall
  ;[1 1 1] spawn shot
  (bind _returnvalue (Game|SpawnActorfromClass (Variables|Default|Getshot) (Transformation|GetActorTransform) "Undefined" "SelectDefaultAtRuntime" 0 0))
  ;[1 1 1] repeat control
  (Utilities|FlowControl|Delay 2.0)
  (Utilities|IsValid _returnvalue
    (:Is%20Valid
      ;[1 1 1] destroy
      (Actor|DestroyActor _returnvalue))))

(event EventBeginPlay
  (|CallParentFunction)
  (Transformation|AttachComponentToComponent (Variables|Default|GetCasting) (Variables|Character|GetMesh) "CastingPoint" "KeepRelative" "KeepRelative" "KeepRelative" true))

(event Collision|EventActorBeginOverlap
  (params (OtherActor :type Actor%20Object%20Reference))
  (|CallParentFunction OtherActor) ; 지금 이 노드는 비활성 상태입니다. \n핀을 끌어서 다른 노드를 연결하면 활성화됩니다.
)

(event EventTick
  (params (DeltaSeconds :type Float%20%28single-precision%29))
  (|CallParentFunction DeltaSeconds) ; 지금 이 노드는 비활성 상태입니다. \n핀을 끌어서 다른 노드를 연결하면 활성화됩니다.
)

(fn ConstructionScript
  (|CallParentFunction))