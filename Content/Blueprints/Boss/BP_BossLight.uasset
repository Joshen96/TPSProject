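; BP_BossLight is a timed boss area attack with a decal warning.
; Tick drives the decal's dynamic material "present" parameter from elapsed time, scaled by its "MaxPresent" value, until it reaches 0.5.
; It then fires once: plays a sound, hides the decal, activates particles, briefly enables sphere collision and destroys itself.
; A TPSPlayer beginning overlap with the sphere receives OnHitEvent.
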(event OnComponentBeginOverlap(Sphere)
  (params (OverlappedComponent :type Primitive%20Component%20Object%20Reference) (OtherActor :type Actor%20Object%20Reference) (OtherComp :type Primitive%20Component%20Object%20Reference) (OtherBodyIndex :type Integer) (bFromSweep :type Boolean) (SweepResult :type Hit%20Result%20Structure%20%28by%20ref%29))
  (bind _astpsplayer (Utilities|Casting|CastToTPSPlayer OtherActor))
  (Class|TPSPlayer|OnHitEvent _astpsplayer 2))

(event EventBeginPlay
  (bind _returnvalue (Rendering|Material|CreateDynamicMaterialInstance (Variables|Default|GetDecal) :!class /Script/Engine.DecalComponent))
  (bind _output_get (Variables|Default|SetDecalSet _returnvalue))
  (bind _returnvalue_2 (Rendering|Material|GetScalarParameterValue _output_get "MaxPresent" :!class /Script/Engine.MaterialInstanceDynamic))
  (Variables|Default|SetMaxPersent _returnvalue_2))

(event Collision|EventActorBeginOverlap
  (params (OtherActor :type Actor%20Object%20Reference)))

(event EventTick
  (params (DeltaSeconds :type Float%20%28single-precision%29))
  (bind _sphere (Variables|Default|GetSphere))
  (bind _output_get (Variables|Default|SetNowTime (+ DeltaSeconds (Variables|Default|GetNowTime))))
  (bind _output_get_2 (Variables|Default|SetCurrentPerSent (* (/ _output_get (Variables|Default|GetmaxCount)) (Variables|Default|GetMaxPersent))))
  (if (< _output_get_2 0.5)
    (Rendering|Material|SetScalarParameterValue (Variables|Default|GetDecalSet) "present" _output_get_2 :!class /Script/Engine.MaterialInstanceDynamic)
    (else
      (Utilities|FlowControl|DoOnce false
        (:Completed
          (Audio|PlaySoundatLocation "/Game/Blueprints/Boss/BossAnim/BossSound/designed-fire-impacts-complex-04-118165_D_major__bpm_144.designed-fire-impacts-complex-04-118165_D_major__bpm_144" (Transformation|GetActorLocation) "0, 0, 0" 1.0 1.0 0.0 0 0 0 0)
          (Rendering|SetVisibility (Variables|Default|GetDecal) false false)
          (Components|Activation|SetActive (Variables|Default|GetParticleSystem) true false)
          (Collision|SetCollisionProfileName _sphere "EnemyKick" true :!class /Script/Engine.PrimitiveComponent)
          (Utilities|FlowControl|Delay 0.2)
          (Collision|SetCollisionProfileName _sphere "NoCollision" true :!class /Script/Engine.PrimitiveComponent)
          (Utilities|FlowControl|Delay 0.5)
          (Actor|DestroyActor))))))

(fn ConstructionScript)