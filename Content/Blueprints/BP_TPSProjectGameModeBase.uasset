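; Game mode for the TPS project that tracks enemy population, kills and weapon unlock progress.
; Tick broadcasts a spawn lock while the living enemy total is at or above a cap, and an unlock otherwise.
; Each enemy death updates the totals and counts down the missile, sub-gun and shield counters, broadcasting each unlock when its counter hits zero.
; It also relays the magnetic soul event with an actor reference.
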(event Custom|Call%20MagneticSoul
  (params (Actor :type Actor%20Object%20Reference))
  (Default|CallMagneticSoul Actor))

(event EventBeginPlay
  (Variables|Default|SetEnemyKillCount 0))

(event EventTick
  (params (DeltaSeconds :type Float%20%28single-precision%29))
  (if (>= (Variables|Default|GetEnemyTotal) 30)
    (Default|CallEnemySpawnLock)
    (else
      (Default|CallEnemySpawnUnLock))))

(fn ConstructionScript)

(fn FEnemyDieCount
  (Variables|Default|SetEnemyTotal (- (Variables|Default|GetEnemyTotal) 1))
  (Variables|Default|SetEnemyKillCount (+ (Variables|Default|GetEnemyKillCount) 1))
  (Variables|Default|SetUnLockMissileCount (- (Variables|Default|GetUnLockMissileCount) 1))
  (Variables|Default|SetUnLockSubGunCount (- (Variables|Default|GetUnLockSubGunCount) 1))
  (Variables|Default|SetUnLockShieldCount (- (Variables|Default|GetUnLockShieldCount) 1))
  (CallFunction|FKillCheck))

(fn FEnemyTotalCount
  (Variables|Default|SetEnemyTotal (+ (Variables|Default|GetEnemyTotal) 1)))

(fn FMissileUnLock
  (Default|CallMissileUnLock))

(fn FKillCheck
  (Utilities|FlowControl|Sequence
    (:then_0
      (if (== (Variables|Default|GetUnLockMissileCount) 0)
        (CallFunction|FMissileUnLock)))
    (:then_1
      (if (== (Variables|Default|GetUnLockSubGunCount) 0)
        (CallFunction|FSubGunUnLock)))
    (:then_2
      (if (== (Variables|Default|GetUnLockShieldCount) 0)
        (CallFunction|FShieldUnLock)))))

(fn FSubGunUnLock
  (Default|CallSubGunUnLock))

(fn FShieldUnLock
  (Default|CallShieldUnLock))