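; BP_Boss is a boss Blueprint that provides two timeline-driven motion events, while its default events and construction script stay empty.
; Forward restarts a timeline that nudges the actor along its forward vector, lerping each update from its current location toward a point slightly ahead.
; LockAtLerp plays a second timeline that turns the actor from its current rotation toward the Target actor, recomputing the look-at rotation each update.
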(event Custom|Forward
  (bind _newtrack_0 (Timeline|타임라인 PlayFromStart)
    (:Update
      (Transformation|SetActorLocation (Math|Vector|Lerp(Vector) (Transformation|GetActorLocation) (+ (Transformation|GetActorLocation) (* (Transformation|GetActorForwardVector) 1e+01)) _newtrack_0) false false))))

(event Custom|LockAtLerp
  (bind _newtrack_0 (Timeline|타임라인_0 Play)
    (:Update
      (Transformation|SetActorRotation (Math|Rotator|Lerp(Rotator) (Transformation|GetActorRotation) (Math|Rotator|FindLookatRotation (Transformation|GetActorLocation) (Transformation|GetActorLocation (Variables|Default|Gettarget))) _newtrack_0)))))

(event EventBeginPlay)

(event Collision|EventActorBeginOverlap
  (params (OtherActor :type Actor%20Object%20Reference)))

(event EventTick
  (params (DeltaSeconds :type Float%20%28single-precision%29)))

(fn ConstructionScript)