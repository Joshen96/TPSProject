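; Enemy actor Blueprint handling health bar, hit feedback, kick hitbox and death.
; BeginPlay links the health bar widget and finds BP_SoundManager; Hit plays sound and reveals the bar once, while CreateDamageUI spawns jittered floating damage text.
; Attackstart and Attackend toggle the Kick collision profile to open and close the attack window.
; SpawnExp runs once, playing death sound and dropping BP_Soul, then, if Fsm state is Die, hiding the bar and destroying the actor after a delay.
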(event Custom|SetupWidgets
  (CallFunction|CreatHeathWidget))

(event EventBeginPlay
  (bind _aswb_enemy_health_bar (Utilities|Casting|CastToWB_EnemyHealthBar (UserInterface|GetUserWidgetObject (Variables|Default|GetHealthWidget))))
  (Variables|/Game/Blueprints/UI/WB_EnemyHealthBar.WB_EnemyHealthBar_C|SetOwnerActor _aswb_enemy_health_bar self)
  (bind _returnvalue (Actor|GetActorOfClass "/Game/Blueprints/SoundManager/BP_SoundManager.BP_SoundManager_C"))
  (Variables|Default|SetSoundManager _returnvalue))

(event Collision|EventActorBeginOverlap
  (params (OtherActor :type Actor%20Object%20Reference)))

(event EventHit
  (Default|EnemyHitSound (Variables|Default|GetSoundManager) (Transformation|GetActorLocation))
  (Utilities|FlowControl|DoOnce false
    (:Completed
      (Rendering|SetVisibility (Variables|Default|GetHealthWidget) true false))))

(event EventCreateDamageUI
  (params (_Damage :type Integer))
  (Game|SpawnActorfromClass "/Game/Blueprints/BP_FloatingText.BP_FloatingText_C" (Math|Transform|MakeTransform (+ (Transformation|GetActorLocation) (Math|Vector|MakeVector (Math|Random|RandomFloatinRange -2e+01 2e+01) (Math|Random|RandomFloatinRange -2e+01 2e+01) (Math|Random|RandomFloatinRange -2e+01 2e+01))) "0, 0, 0" "0.0,0.0,0.0") "Undefined" "MultiplyWithRoot" 0 (Math|Conversions|ToFloat(Integer) _Damage) 0))

(event EventTick
  (params (DeltaSeconds :type Float%20%28single-precision%29)))

(event EventKillCount
  (Default|CallEnemyDie))

(event EventSpawnExp
  (bind _returnvalue (Transformation|GetActorLocation))
  (Utilities|FlowControl|DoOnce false
    (:Completed
      (Default|EnemyDieSound (Variables|Default|GetSoundManager) _returnvalue)
      (Game|SpawnActorfromClass "/Game/Blueprints/Items/BP_Soul.BP_Soul_C" (Math|Transform|MakeTransform _returnvalue "0, 0, 0" "1.000000,1.000000,1.000000") "Undefined" "MultiplyWithRoot" 0 0)
      (if (Utilities|Enum|Equal(Enum) (Variables|/Script/TPSProject.EnemyFSM|GetmState (Variables|Default|Getfsm)) "Die")
        (Utilities|FlowControl|DoOnce false
          (:Completed
            (Rendering|SetVisibility (Variables|Default|GetHealthWidget) false false)
            (Collision|SetCollisionEnabled (Variables|Default|Getkick) "NoCollision")
            (Utilities|FlowControl|Delay 1.0)
            (Actor|DestroyActor)))))))

(event EventSetupHealthWidget)

(event EventAttackend
  (Collision|SetCollisionProfileName (Variables|Default|Getkick) "NoCollision" true :!class /Script/Engine.PrimitiveComponent))

(event EventAttackstart
  (Collision|SetCollisionProfileName (Variables|Default|Getkick) "EnemyKick" true :!class /Script/Engine.PrimitiveComponent))

(fn ConstructionScript)

(fn CreatHeathWidget
  (bind _fsm (Variables|Default|Getfsm))
  (bind _returnvalue (UserInterface|CreateWidget "/Game/Blueprints/UI/WB_EnemyHealthBar.WB_EnemyHealthBar_C"))
  (bind _output_get (Variables|FSMComponent|SetEnemyHealthBarWidgetReference _returnvalue))
  (Progress|SetPercent (Variables|/Game/Blueprints/UI/WB_EnemyHealthBar.WB_EnemyHealthBar_C|GetProgressBar_1 _output_get) (/ (Math|Conversions|ToFloat(Integer) (Variables|/Script/TPSProject.EnemyFSM|GetcurrntHp _fsm)) (Math|Conversions|ToFloat(Integer) (Variables|/Script/TPSProject.EnemyFSM|GetmaxHp _fsm))))
  (return))

(fn NewFunction)