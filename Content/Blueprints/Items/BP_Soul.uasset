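; BP_Soul is an XP pickup that flies to the player and grants experience.
; Outer Sphere overlap with BP_TPSPlayer stores the player and starts a one-time timeline lerp toward their live location.
; BeginPlay also binds the first found BP_MagnetItem's event to a second, similar pull timeline.
; Any Inner collision overlap spawns an ice particle, then passes XPAmount to the stored player's PlayerLevelUp once and destroys the soul.
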(event OnComponentBeginOverlap(Sphere)
  (params (OverlappedComponent :type Primitive%20Component%20Object%20Reference) (OtherActor :type Actor%20Object%20Reference) (OtherComp :type Primitive%20Component%20Object%20Reference) (OtherBodyIndex :type Integer) (bFromSweep :type Boolean) (SweepResult :type Hit%20Result%20Structure%20%28by%20ref%29))
  ;[0.1094 0.1094 0.1094] 외각 콜리전에 다이면 흡수
  (bind _asbp_tpsplayer (Utilities|Casting|CastToBP_TPSPlayer OtherActor))
  (Utilities|FlowControl|DoOnce false
    (:Completed
      (Variables|Default|SetPlayer _asbp_tpsplayer)
      (Variables|Default|SetStarting%20Location (Transformation|GetActorLocation))
      (bind _newtrack_0 (Timeline|Timeline_0 Play)
        (:Update
          (Transformation|SetActorLocation (Math|Vector|Lerp(Vector) (Variables|Default|GetStarting%20Location) (Transformation|GetActorLocation (Variables|Default|GetPlayer)) _newtrack_0) false false))))))

(event OnComponentBeginOverlap(Inner)
  (params (OverlappedComponent :type Primitive%20Component%20Object%20Reference) (OtherActor :type Actor%20Object%20Reference) (OtherComp :type Primitive%20Component%20Object%20Reference) (OtherBodyIndex :type Integer) (bFromSweep :type Boolean) (SweepResult :type Hit%20Result%20Structure%20%28by%20ref%29))
  ;[0.1094 0.1094 0.1094] xp 획득
  (Effects|SpawnEmitteratLocation "/Game/SurvivorsTemplate/Demo/Effects/FX_Mobile/combat/P_ProjectileLob_Ice_Charge_01.P_ProjectileLob_Ice_Charge_01" (Transformation|GetWorldLocation (Variables|Default|GetInner)))
  (CallFunction|AddXP))

(event Custom|AddXP
  ;[0.1094 0.1094 0.1094] xp 획득
  (Utilities|FlowControl|DoOnce false
    (:Completed
      (bind _asbp_tpsplayer (Utilities|Casting|CastToBP_TPSPlayer (Variables|Default|GetPlayer)))
      (Default|PlayerLevelUp _asbp_tpsplayer (Variables|Default|GetXPAmount))
      (Actor|DestroyActor))))

(event Custom|SoulToPlayer
  (params (Player :type Actor%20Object%20Reference))
  ;[1 1 1] 자석 효과 바인딩
  (Variables|Default|SetStarting%20Location (Transformation|GetActorLocation))
  (bind _newtrack_0 (Timeline|타임라인 Play)
    (:Update
      (Transformation|SetActorLocation (Math|Vector|Lerp(Vector) (Variables|Default|GetStarting%20Location) (Transformation|GetActorLocation Player) _newtrack_0) false false))))

(event EventBeginPlay
  (bind _returnvalue (Actor|GetActorOfClass "/Game/Blueprints/Items/BP_MagnetItem.BP_MagnetItem_C"))
  (EventDispatchers|BindEventtoMagneticSoul _returnvalue (delegate Custom|SoulToPlayer)))

(event Collision|EventActorBeginOverlap
  (params (OtherActor :type Actor%20Object%20Reference)))

(event EventTick
  (params (DeltaSeconds :type Float%20%28single-precision%29)))

(fn ConstructionScript)