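; BP_ItemBox is an item box that spawns one random item when its HitZone is first overlapped, then destroys itself.
; The overlap passes through a DoOnce into SpawnRandomItem, which picks a class from ItemList using a hardcoded index range covering three entries.
; It plays a Niagara healing effect at the box location and spawns the chosen item slightly above it at enlarged scale.
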(event OnComponentBeginOverlap(HitZone)
  (params (OverlappedComponent :type Primitive%20Component%20Object%20Reference) (OtherActor :type Actor%20Object%20Reference) (OtherComp :type Primitive%20Component%20Object%20Reference) (OtherBodyIndex :type Integer) (bFromSweep :type Boolean) (SweepResult :type Hit%20Result%20Structure%20%28by%20ref%29))
  (Utilities|FlowControl|DoOnce false
    (:Completed
      (CallFunction|SpawnRandomItem))))

(event EventBeginPlay)

(event Collision|EventActorBeginOverlap
  (params (OtherActor :type Actor%20Object%20Reference)))

(event EventTick
  (params (DeltaSeconds :type Float%20%28single-precision%29)))

(fn ConstructionScript)

(fn SpawnRandomItem
  (bind _returnvalue (Transformation|GetActorLocation))
  (bind _output_get (Variables|Default|Setset (Math|Random|RandomIntegerinRange 0 2)))
  (Niagara|SpawnSystematLocation "/Game/sA_PickupSet_1/Fx/NiagaraSystems/NS_Healing_3.NS_Healing_3" _returnvalue "0, 0, 0" "2.000000,2.000000,2.000000")
  (Game|SpawnActorfromClass (Utilities|Array|Get(acopy) (Variables|Default|GetItemList) _output_get) (Math|Transform|MakeTransform (+ _returnvalue "0.000000,0.000000,30.000000") "0, 0, 0" "2.000000,2.000000,2.000000") "Undefined" "MultiplyWithRoot" 0 0)
  (Actor|DestroyActor))