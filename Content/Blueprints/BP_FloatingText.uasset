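; BP_FloatingText is an actor that shows a floating damage number.
; On BeginPlay it writes the truncated Damage value as an integer into the HitDamageUI text block of its widget component.
; One timeline fades the text's opacity while a second lerps the actor 75 units upward from its spawn location, then destroys it when finished.
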(event EventBeginPlay
  ;[1 1 1] Fade Out
  (Utilities|FlowControl|Sequence
    (:then_0
      (bind _ashit_damage_ui (Utilities|Casting|CastToHitDamageUI (UserInterface|GetUserWidgetObject (Variables|Default|GetWidget))))
      (Rendering|Components|TextRender|SetText (Variables|/Game/Blueprints/HitDamageUI.HitDamageUI_C|GetTextBlock_Damage _ashit_damage_ui) (Utilities|Text|ToText(Integer) (Math|Float|Truncate (Variables|Default|GetDamage))))
      (bind _새_트랙_0 (Timeline|fade PlayFromStart)
        (:Update
          (Widget|SetRenderOpacity (Variables|/Game/Blueprints/HitDamageUI.HitDamageUI_C|GetTextBlock_Damage _ashit_damage_ui) _새_트랙_0))))
    (:then_1
      ;[1 1 1] Move Up
      (Variables|Default|SetInitialLocation (Transformation|GetActorLocation))
      (bind _새_트랙_0_2 (Timeline|타임라인_0 PlayFromStart)
        (:Update
          (Transformation|SetActorLocation (Math|Vector|Lerp(Vector) (Variables|Default|GetInitialLocation) (+ (Variables|Default|GetInitialLocation) "0.000000,0.000000,75.000000") _새_트랙_0_2) false false))
        (:Finished
          ;[1 1 1] Destroy when done
          (Actor|DestroyActor))))))

(fn ConstructionScript)