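; Homing missile weapon Blueprint that damages enemies overlapping its HitBox by passing its damage value to the enemy's FSM.
; BeginPlay also binds to GameInstance rotate-delay and sub-power events, with level-up handlers that scale damage and a delay multiplier.
; An endless Delay loop pulses the explosion particle on and off.
; A DoOnce-guarded PlaySound event plays a launch sound, then a hit sound at the actor's location.
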(event Custom|OnComponentBeginOverlap_이벤트
  (params (OverlappedComponent :type Primitive%20Component%20Object%20Reference) (OtherActor :type Actor%20Object%20Reference) (OtherComp :type Primitive%20Component%20Object%20Reference) (OtherBodyIndex :type Integer) (bFromSweep :type Boolean) (SweepResult :type Hit%20Result%20Structure%20%28by%20ref%29))
  ;[1 1 1] 적을 타격시 데미지주기
  (bind _asenemy (Utilities|Casting|CastToEnemy OtherActor))
  (Utilities|Casting|CastToEnemyFSMClass "/Script/TPSProject.EnemyFSM")
  (Class|EnemyFSM|OnDamageProcess (Variables|/Script/TPSProject.Enemy|Getfsm _asenemy) (Math|Float|Truncate (Variables|Default|GetDamageHoming))))

(event Custom|PlaySound
  ;[1 1 1] 사운드 실행
  (Utilities|FlowControl|DoOnce false
    (:Completed
      (Audio|PlaySound2D "/Game/Sound/launch-sequence-81945__cut_2sec_.launch-sequence-81945__cut_2sec_" 1.0 1.0 0.0 0 0)
      (Utilities|FlowControl|Delay 0.5)
      (Audio|PlaySoundatLocation (Variables|Default|GetHitSound) (Transformation|GetActorLocation) "0, 0, 0" 1.0 1.0 0.0 0 0 0 0))))

(event Custom|MissilePowerUp
  (params (DamgeSetting :type Float%20%28double-precision%29))
  ;[1 1 1] 레벨업을 통한 효과변경
  (Variables|Default|SetDamageHoming (* (Variables|Default|GetDamageHoming) DamgeSetting)))

(event Custom|MissileDelay
  (params (delaySetting :type Float%20%28double-precision%29))
  ;[1 1 1] 레벨업을 통한 효과변경
  (Variables|Default|SetMultiplier (* (Variables|Default|GetMultiplier) delaySetting)))

(event EventBeginPlay
  (bind _particlesystem (Variables|Default|GetParticleSystem))
  (Collision|AssignOnComponentBeginOverlap (Variables|Default|GetHitBox) (delegate Custom|OnComponentBeginOverlap_이벤트))
  (bind _asgi_game_instance (Utilities|Casting|CastToGI_GameInstance (Game|GetGameInstance)))
  (EventDispatchers|BindEventtoRotateDelay _asgi_game_instance (EventDispatchers|CreateEvent :!event Custom|MissileDelay))
  (EventDispatchers|BindEventtoSubPower _asgi_game_instance (EventDispatchers|CreateEvent :!event Custom|MissilePowerUp))
  ;[1 1 1] 터지는 이펙트 루프
  (Components|Activation|Activate _particlesystem false :!label _label)
  (Utilities|FlowControl|Delay 0.5)
  (Components|Activation|Deactivate _particlesystem)
  (goto _label))

(event Collision|EventActorBeginOverlap
  (params (OtherActor :type Actor%20Object%20Reference)))

(event EventTick
  (params (DeltaSeconds :type Float%20%28single-precision%29)))

(fn ConstructionScript)