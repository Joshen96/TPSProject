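; Game instance that holds player progression: level, EXP threshold and per-skill levels.
; LevelUP raises the level, scales the EXP threshold by a multiplier, then caches references to the TPS player and the missile system actor.
; SkillUP increments the indexed skill level and dispatches the matching upgrade (basic gun power, sub gun delay, health or missile power) through those cached references.
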(event Custom|LevelUP
  (Variables|Default|SetPlayerLV (+ (Variables|Default|GetPlayerLV) 1))
  (Variables|Default|SetPlayerEXPMax (* (Variables|Default|GetPlayerEXPMax) (Variables|Default|GetExpMultiplier)))
  (bind _asbp_tpsplayer (Utilities|Casting|CastToBP_TPSPlayer (Game|GetPlayerCharacter 0)))
  (Variables|Default|SetPlayer _asbp_tpsplayer)
  (bind _returnvalue (Actor|GetActorOfClass "/Game/Blueprints/Target2.Target2_C"))
  (Variables|Default|SetMissileSystem _returnvalue))

(event Custom|SkillUP
  (params (index :type Integer))
  (bind _player (Variables|Default|GetPlayer))
  (bind _skilllevel (Variables|Default|GetSkillLevel))
  (bind _output (Utilities|Array|Get(acopy) _skilllevel index))
  (Utilities|ManipulateIntInternal _output (+ _output 1)
    (:%20%20
      (switch int index
        (:0
          (Default|BasicGunPowerUp _player))
        (:1
          (Default|SubGunDelayUp _player))
        (:2
          (Default|PlayerHeathUp _player))
        (:3
          (Default|MissilePowerUp (Variables|Default|GetMissileSystem)))))))