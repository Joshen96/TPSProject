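; Enemy Blueprint that handles health bar, kick hitbox, damage numbers, soul drop and kill notification around an Fsm state component.
; OC/MC-prefixed events create the widget and update its bar from HP percent.
; Tick polls the FSM state to reveal the bar on damage and toggle Kick collision.
; Events spawn floating text and a one-time BP_Soul, hiding the bar and disabling Kick on death, and call EnemyDie.
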(event Custom|SetupWidgets)

(event Custom|MC_UpdateHealthBar
  (params (Percent :type Float%20%28double-precision%29))
  (bind _enemyhealthbarwidgetreference (Variables|FSMComponent|GetEnemyHealthBarWidgetReference)
    (:then
      (Progress|SetPercent (Variables|/Game/Blueprints/WB_EnemyHealthBar.WB_EnemyHealthBar_C|GetProgressBar_1 _enemyhealthbarwidgetreference) Percent))
    (:else)))

(event Custom|OC_SetupWidgets
  (CallFunction|CreatHeathWidget))

(event EventBeginPlay)

(event Collision|EventActorBeginOverlap
  (params (OtherActor :type Actor%20Object%20Reference)))

(event EventCreateDamageUI
  (params (_Damage :type Integer))
  (Game|SpawnActorfromClass "/Game/Blueprints/BP_FloatingText.BP_FloatingText_C" (Math|Transform|MakeTransform (+ (Transformation|GetActorLocation) (Math|Vector|MakeVector 0.0 0.0 0.0)) "0, 0, 0" "1.000000,1.000000,1.000000") "Undefined" "MultiplyWithRoot" 0 (Math|Conversions|ToFloat(Integer) _Damage) 0))

(event EventTick
  (params (DeltaSeconds :type Float%20%28single-precision%29))
  (bind _kick (Variables|Default|Getkick))
  (if (Utilities|Enum|Equal(Enum) (Variables|/Script/TPSProject.EnemyFSM|GetmState (Variables|Default|Getfsm)) "Damage")
    (Rendering|SetVisibility (Variables|Default|GetHealthWidget) true false))
  (if (== (Variables|/Script/TPSProject.EnemyFSM|GetmState (Variables|Default|Getfsm)) 2)
    (Collision|SetCollisionProfileName _kick "EnemyKick" true :!class /Script/Engine.PrimitiveComponent)
    (else
      (Collision|SetCollisionProfileName _kick "NoCollision" true :!class /Script/Engine.PrimitiveComponent))))

(event EventKillCount
  (Default|CallEnemyDie))

(event EventSpawnExp
  (Utilities|FlowControl|DoOnce false
    (:Completed
      (Game|SpawnActorfromClass "/Game/Blueprints/Items/BP_Soul.BP_Soul_C" (Math|Transform|MakeTransform (+ (Transformation|GetActorLocation) "0.000000,0.000000,30.000000") "0, 0, 0" "1.000000,1.000000,1.000000") "Undefined" "MultiplyWithRoot" 0 0)
      (if (Utilities|Enum|Equal(Enum) (Variables|/Script/TPSProject.EnemyFSM|GetmState (Variables|Default|Getfsm)) "Die")
        (Utilities|FlowControl|DoOnce false
          (:Completed
            (Rendering|SetVisibility (Variables|Default|GetHealthWidget) false false)
            (Collision|SetCollisionEnabled (Variables|Default|Getkick) "NoCollision")))))))

(event EventSetupHealthWidget)

(fn ConstructionScript)

(fn CreatHeathWidget
  (bind _fsm (Variables|Default|Getfsm))
  (bind _returnvalue (UserInterface|CreateWidget "/Game/Blueprints/WB_EnemyHealthBar.WB_EnemyHealthBar_C"))
  (bind _output_get (Variables|FSMComponent|SetEnemyHealthBarWidgetReference _returnvalue))
  (UserInterface|SetWidget (Variables|Default|GetHealthWidget) _output_get)
  (CallFunction|MCUpdateHealthBar (/ (Math|Conversions|ToFloat(Integer) (Variables|/Script/TPSProject.EnemyFSM|GetcurrntHp _fsm)) (Math|Conversions|ToFloat(Integer) (Variables|/Script/TPSProject.EnemyFSM|GetmaxHp _fsm)))))

(fn NewFunction
  (Variables|Default|SetProgressBar1 0))