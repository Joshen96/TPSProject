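; BP_Enemy1 is an enemy actor that displays its health bar and floating damage numbers.
; On BeginPlay or a setup event, it creates WB_EnemyHealthBar, assigns it to its HealthWidget component and fills it from the Fsm1 component's current-to-max HP ratio.
; MC_UpdateHealthBar sets the progress bar percent, and CreateDamageUI spawns BP_FloatingText with the damage value at a slightly randomized offset from the enemy.
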(event Custom|CreateDamageUI
  (params (Damage :type Float%20%28double-precision%29))
  (Game|SpawnActorfromClass "/Game/Blueprints/BP_FloatingText.BP_FloatingText_C" (Math|Transform|MakeTransform (+ (Transformation|GetActorLocation) (Math|Vector|MakeVector (Math|Random|RandomFloatinRange -1e+01 1e+01) (Math|Random|RandomFloatinRange -1e+01 1e+01) (Math|Random|RandomFloatinRange -1e+01 1e+01))) "0, 0, 0" "1.000000,1.000000,1.000000") "Undefined" "MultiplyWithRoot" 0 Damage 0))

(event Custom|SetupWidgets
  (CallFunction|OCSetupWidgets))

(event Custom|MC_UpdateHealthBar
  (params (Percent :type Float%20%28double-precision%29))
  (bind _enemyhealthbarwidgetreference (Variables|FSMComponent|GetEnemyHealthBarWidgetReference)
    (:then
      (Progress|SetPercent (Variables|/Game/Blueprints/WB_EnemyHealthBar.WB_EnemyHealthBar_C|GetProgressBar_1 _enemyhealthbarwidgetreference) Percent))
    (:else)))

(event Custom|OC_SetupWidgets
  (CallFunction|CreatHeathWidget))

(event EventBeginPlay
  (CallFunction|OCSetupWidgets))

(event Collision|EventActorBeginOverlap
  (params (OtherActor :type Actor%20Object%20Reference)))

(event EventTick
  (params (DeltaSeconds :type Float%20%28single-precision%29)))

(event EventSetupHealthWidget
  (CallFunction|OCSetupWidgets))

(fn ConstructionScript)

(fn CreatHeathWidget
  (bind _fsm1 (Variables|Default|Getfsm1))
  (bind _returnvalue (UserInterface|CreateWidget "/Game/Blueprints/WB_EnemyHealthBar.WB_EnemyHealthBar_C"))
  (bind _output_get (Variables|FSMComponent|SetEnemyHealthBarWidgetReference _returnvalue))
  (UserInterface|SetWidget (Variables|Default|GetHealthWidget) _output_get)
  (CallFunction|MCUpdateHealthBar (/ (Math|Conversions|ToFloat(Integer) (Variables|/Script/TPSProject.EnemyFSM|GetcurrntHp _fsm1)) (Math|Conversions|ToFloat(Integer) (Variables|/Script/TPSProject.EnemyFSM|GetmaxHp _fsm1)))))

(fn NewFunction
  (Variables|Default|SetProgressBar1 0))

(fn CustomEvent)

(fn CustomEvent1)