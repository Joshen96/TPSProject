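; Target2 is a damage-zone actor, apparently a homing missile's target effect, that hurts enemies entering its HitBox.
; BeginPlay binds the overlap, which passes truncated DamageHoming to the enemy FSM's OnDamageProcess.
; It then runs the particle system in half-second cycles while IsLoop is set, otherwise destroying itself after the first.
; MissilePowerUp scales the damage up, and PlaySound plays a one-time launch sound followed by a delayed hit sound.
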(event Custom|OnComponentBeginOverlap_이벤트
  (params (OverlappedComponent :type Primitive%20Component%20Object%20Reference) (OtherActor :type Actor%20Object%20Reference) (OtherComp :type Primitive%20Component%20Object%20Reference) (OtherBodyIndex :type Integer) (bFromSweep :type Boolean) (SweepResult :type Hit%20Result%20Structure%20%28by%20ref%29))
  (bind _asenemy (Utilities|Casting|CastToEnemy OtherActor))
  (Utilities|Casting|CastToEnemyFSMClass "/Script/TPSProject.EnemyFSM")
  (Class|EnemyFSM|OnDamageProcess (Variables|/Script/TPSProject.Enemy|Getfsm _asenemy) (Math|Float|Truncate (Variables|Default|GetDamageHoming))))

(event Custom|PlaySound
  (Utilities|FlowControl|DoOnce false
    (:Completed
      (Audio|PlaySound2D "/Game/Sound/launch-sequence-81945__cut_2sec_.launch-sequence-81945__cut_2sec_" 1.0 1.0 0.0 0 0)
      (Utilities|FlowControl|Delay 1.0)
      (Audio|PlaySoundatLocation (Variables|Default|GetHitSound) (Transformation|GetActorLocation) "0, 0, 0" 1.0 1.0 0.0 0 0 0 0))))

(event Custom|MissilePowerUp
  (Variables|Default|SetDamageHoming (* (Variables|Default|GetDamageHoming) 1.2)))

(event EventBeginPlay
  (bind _particlesystem (Variables|Default|GetParticleSystem))
  (Collision|AssignOnComponentBeginOverlap (Variables|Default|GetHitBox) (delegate Custom|OnComponentBeginOverlap_이벤트))
  (Components|Activation|Activate _particlesystem false :!label _label)
  (Utilities|FlowControl|Delay 0.5)
  (if (Variables|Default|GetisLoop)
    (Components|Activation|Deactivate _particlesystem)
    (goto _label)
    (else
      (Actor|DestroyActor))))

(event Collision|EventActorBeginOverlap
  (params (OtherActor :type Actor%20Object%20Reference)))

(event EventTick
  (params (DeltaSeconds :type Float%20%28single-precision%29)))

(fn ConstructionScript)