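; BP_Portal1 is a level-transition portal that sends the player to the FirstStageRed level.
; On BeginPlay, a timeline scales it toward 3x, lerping from its current scale on each update.
; When a TPSPlayer overlaps PortalColl, it calls InitState on the project game mode and the game instance, then opens the level by name.
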(event OnComponentBeginOverlap(PortalColl)
  (params (OverlappedComponent :type Primitive%20Component%20Object%20Reference) (OtherActor :type Actor%20Object%20Reference) (OtherComp :type Primitive%20Component%20Object%20Reference) (OtherBodyIndex :type Integer) (bFromSweep :type Boolean) (SweepResult :type Hit%20Result%20Structure%20%28by%20ref%29))
  (Utilities|Casting|CastToTPSPlayer OtherActor)
  (Utilities|FlowControl|Sequence
    (:then_0
      (bind _asbp_tpsproject_game_mode_base (Utilities|Casting|CastToBP_TPSProjectGameModeBase (Game|GetGameMode)))
      (Default|InitState _asbp_tpsproject_game_mode_base))
    (:then_1
      (bind _asgi_game_instance (Utilities|Casting|CastToGI_GameInstance (Game|GetGameInstance)))
      (Default|InitState _asgi_game_instance)
      (Game|OpenLevel(byName) "FirstStageRed"))))

(event EventBeginPlay
  (bind _새_트랙_0 (Timeline|타임라인 PlayFromStart)
    (:Update
      (Transformation|SetActorScale3D (Math|Vector|Lerp(Vector) (Transformation|GetActorScale3D) "3.000000,3.000000,3.000000" _새_트랙_0)))))

(event Collision|EventActorBeginOverlap
  (params (OtherActor :type Actor%20Object%20Reference)))

(event EventTick
  (params (DeltaSeconds :type Float%20%28single-precision%29)))

(fn ConstructionScript)