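; Enemy manager that links enemy spawning and kill counting to BP_TPSProjectGameModeBase.
; On BeginPlay it binds to game mode events that toggle SpawnLock or enable the DistanceEnemySpawn flag for ranged enemies.
; CountEnemyEvent, called when an enemy spawns, increments the game mode's total and observes that BP_Enemy's death event to report kills back.
; The spawn logic that reads these flags is outside this graph.
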(event Custom|SpwanLock
  ;[1 1 1] 애너미 스폰 제한 바인딩
  (Variables|Default|SetbSpawnLock true))

(event Custom|EnemyDieCount
  ;[1 1 1] 생성된 애너미에 죽으면 카운트 하는 이벤트 탑재 (옵저버활용)
  (Default|FEnemyDieCount (stale EventCountEnemyEvent _asbp_tpsproject_game_mode_base)))

(event Custom|SpawnUnLock
  ;[1 1 1] 애너미 스폰 제한 해제 바인딩
  (Variables|Default|SetbSpawnLock false))

(event Custom|DistanceEnemySpawn
  ;[1 1 1] 원거리적 소환 바인딩
  (Variables|Default|SetbDistanceEnemySpawn true))

(event EventBeginPlay
  (bind _asbp_tpsproject_game_mode_base (Utilities|Casting|CastToBP_TPSProjectGameModeBase (Game|GetGameMode)))
  ;[1 1 1] 애너미 스폰 제한 바인딩
  (EventDispatchers|BindEventtoEnemySpawnLock _asbp_tpsproject_game_mode_base (delegate Custom|SpwanLock))
  ;[1 1 1] 애너미 스폰 제한 해제 바인딩
  (EventDispatchers|BindEventtoEnemySpawnUnLock _asbp_tpsproject_game_mode_base (delegate Custom|SpawnUnLock))
  ;[1 1 1] 원거리적 소환 바인딩
  (EventDispatchers|BindEventtoDistanceEnemySpawn _asbp_tpsproject_game_mode_base (delegate Custom|DistanceEnemySpawn)))

(event Collision|EventActorBeginOverlap
  (params (OtherActor :type Actor%20Object%20Reference)))

(event EventTick
  (params (DeltaSeconds :type Float%20%28single-precision%29)))

(event EventCountEnemyEvent
  (params (EnemyOBJ :type Enemy%20Object%20Reference))
  ;[1 1 1] 애너미 생성시자동 호출되는 함수, 적의수 카운트
  (bind _asbp_tpsproject_game_mode_base (Utilities|Casting|CastToBP_TPSProjectGameModeBase (Game|GetGameMode)))
  (Default|FEnemyTotalCount _asbp_tpsproject_game_mode_base)
  ;[1 1 1] 생성된 애너미에 죽으면 카운트 하는 이벤트 탑재 (옵저버활용)
  (bind _asbp_enemy (Utilities|Casting|CastToBP_Enemy EnemyOBJ))
  (EventDispatchers|BindEventtoEnemyDie _asbp_enemy (delegate Custom|EnemyDieCount)))

(fn ConstructionScript)