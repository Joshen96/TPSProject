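; Third-person shooter player Blueprint that drives the HUD, progression and game-over flow.
; XP accumulates in the game instance; leveling pauses play for a skill widget, backed by stat upgrade events for damage, grenade delay, health and speed.
; Tick uses DoOnce to catch shield and sub-gun unlocks, granting them and showing pause popups.
; Enemy ball overlaps trigger hits, and a homing missile event reveals a target actor and feeds its location to Niagara.
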(event Custom|Skillchoose
  (Widget|RemovefromParent (stale Custom|PlayerLevelUp _returnvalue))
  (Variables|/Script/Engine.PlayerController|SetbShowMouseCursor (Game|GetPlayerController 0) false))

(event Custom|PlayerLevelUp
  (params (XP :type Float%20%28double-precision%29))
  (bind _asgi_game_instance (Utilities|Casting|CastToGI_GameInstance (Game|GetGameInstance)))
  (if (< (Variables|/Game/Blueprints/GI_GameInstance.GI_GameInstance_C|GetPlayerEXPMax _asgi_game_instance) (+ XP (Variables|/Game/Blueprints/GI_GameInstance.GI_GameInstance_C|GetCurrentEXP _asgi_game_instance)))
    (Variables|/Game/Blueprints/GI_GameInstance.GI_GameInstance_C|SetCurrentEXP _asgi_game_instance (- (+ XP (Variables|/Game/Blueprints/GI_GameInstance.GI_GameInstance_C|GetCurrentEXP _asgi_game_instance)) (Variables|/Game/Blueprints/GI_GameInstance.GI_GameInstance_C|GetPlayerEXPMax _asgi_game_instance)))
    (Default|LevelUP _asgi_game_instance)
    (Game|SetGamePaused true)
    (Variables|/Script/Engine.PlayerController|SetbShowMouseCursor (Game|GetPlayerController 0) true)
    (bind _returnvalue (UserInterface|CreateWidget "/Game/Blueprints/WBP_LEVELUP.WBP_LEVELUP_C"))
    (UserInterface|Viewport|AddtoViewport _returnvalue 0)
    (else
      (Variables|/Game/Blueprints/GI_GameInstance.GI_GameInstance_C|SetCurrentEXP _asgi_game_instance (+ XP (Variables|/Game/Blueprints/GI_GameInstance.GI_GameInstance_C|GetCurrentEXP _asgi_game_instance))))))

(event Custom|BasicGunPowerUp
  (Variables|Default|SetBasicGunDamage (* (Variables|Default|GetBasicGunDamage) 1.2)))

(event Custom|SubGunDelayUp
  (Variables|Default|SetSubGunDelay (* (Variables|Default|GetSubGunDelay) 0.9)))

(event Custom|PlayerHeathUp
  (Variables|Default|SetinitiaHp (Math|Float|Truncate (* (Math|Conversions|ToFloat(Integer) (Variables|Default|GetinitiaHp)) 1.2)))
  (Variables|Default|Sethp (Math|Float|Truncate (* (Math|Conversions|ToFloat(Integer) (Variables|Default|Gethp)) 1.2))))

(event Custom|PlayerSpeedUp
  (Variables|Default|SetwalkSpeed (+ (Variables|Default|GetwalkSpeed) 3e+01))
  (Variables|Default|SetrunSpeed (+ (Variables|Default|GetrunSpeed) 1e+02)))

(event Custom|UseHommingMissile
  (bind _target2 (Variables|Default|GetTarget2))
  (Rendering|SetVisibility (Variables|Default|GetNiagara) true false)
  (Variables|Default|SetHommingLock false)
  (Rendering|SetActorHiddenInGame _target2 false)
  (Collision|SetCollisionProfileName (Variables|/Game/Blueprints/Target2.Target2_C|GetHitBox _target2) "Missile" true :!class /Script/Engine.PrimitiveComponent)
  (Default|PlaySound _target2)
  (Niagara|SetNiagaraVariable(Vector3) (Variables|Default|GetNiagara) "Target" (Transformation|GetWorldLocation (Variables|/Script/Engine.Actor|GetRootComponent (Variables|Default|GetTarget2)))))

(event Custom|UseGrenadeUI
  (Class|TPSPlayer|UseGrenadeGun)
  (Game|SetGamePaused true)
  (Variables|/Script/Engine.PlayerController|SetbShowMouseCursor (Game|GetPlayerController 0) true)
  (bind _returnvalue (UserInterface|CreateWidget "/Game/Blueprints/WB_SubGunUnLock.WB_SubGunUnLock_C"))
  (UserInterface|Viewport|AddtoViewport _returnvalue 0))

(event Custom|UseShieldUI
  (Game|SpawnActorfromClass (Variables|Default|GetShieldObject) (Transformation|GetActorTransform) "Undefined" "MultiplyWithRoot" 0 0)
  (Game|SetGamePaused true)
  (Variables|/Script/Engine.PlayerController|SetbShowMouseCursor (Game|GetPlayerController 0) true)
  (bind _returnvalue (UserInterface|CreateWidget "/Game/Blueprints/WB_ShieldUnLock.WB_ShieldUnLock_C"))
  (UserInterface|Viewport|AddtoViewport _returnvalue 0))

(event EventBeginPlay
  (bind _returnvalue (UserInterface|CreateWidget "/Game/Blueprints/ScreenUI.ScreenUI_C" (Game|GetPlayerController 0)))
  (Variables|Default|SetUI_Screen _returnvalue)
  (UserInterface|Viewport|AddtoViewport (Variables|Default|GetUI_Screen) 0)
  (Utilities|FlowControl|Delay 0.05)
  (Class|TPSPlayer|OnUsingGrenade false)
  (Rendering|SetVisibility (Variables|Default|GetNiagara) false false)
  (bind _returnvalue_2 (Actor|GetActorOfClass "/Game/Blueprints/Target2.Target2_C"))
  (Variables|Default|SetTarget2 _returnvalue_2))

(event EventTick
  (params (DeltaSeconds :type Float%20%28single-precision%29))
  (Utilities|FlowControl|Sequence
    (:then_0
      (if (Variables|Default|GetSubGun)
        (Utilities|FlowControl|DoOnce false
          (:Completed
            (CallFunction|UseGrenadeUI)))))
    (:then_1
      (if (Variables|Default|GetShield)
        (Utilities|FlowControl|DoOnce false
          (:Completed
            (CallFunction|UseShieldUI)))))))

(event EventOnGameOver
  (|CallParentFunction)
  (Variables|/Script/Engine.PlayerController|SetbShowMouseCursor (Game|GetPlayerController 0) true)
  (bind _returnvalue (UserInterface|CreateWidget "/Game/Blueprints/UI_GameOver.UI_GameOver_C"))
  (UserInterface|Viewport|AddtoViewport _returnvalue 0))

(event EventOnUsingGrenade
  (params (isGrenade :type Boolean))
  (bind _ui_screen (Variables|Default|GetUI_Screen))
  (Utilities|IsValid _ui_screen
    (:Is%20Valid
      (Variables|/Game/Blueprints/ScreenUI.ScreenUI_C|SetIsGrenaded _ui_screen isGrenade)
      (Default|SwapWeapon _ui_screen))))

(event Collision|EventActorBeginOverlap
  (params (OtherActor :type Actor%20Object%20Reference))
  (Utilities|Casting|CastToBP_EnemyBall OtherActor)
  (Class|TPSPlayer|OnHitEvent))

(event Input|ActionEvents|InputActionSniper
  (params (Key :type Key%20Structure :default "None")))

(fn ConstructionScript)

(fn UIctrlHP)